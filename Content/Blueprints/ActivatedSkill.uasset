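; ActivatedSkill is a base Blueprint for player-activated skills, with an empty Activate event and a helper that computes a spawn transform ahead of the user.
; SetupActivation gates use on an affordability check, then stores the user, roots PlayerCharacters for RootTime and deducts Cost from skill points.
; A second eligibility function has disconnected rooted and airborne checks, so neither restriction applies.
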(event Custom|Activate
  (params (Owner :type Skill%20Consumer%20Object%20Reference)))

(event EventBeginPlay)

(event Collision|EventActorBeginOverlap
  (params (OtherActor :type Actor%20Object%20Reference)))

(event EventTick
  (params (DeltaSeconds :type Float%20%28single-precision%29)))

(fn ConstructionScript)

(fn GetSkillSpawnPoint
  (params (User :type Skill%20Consumer%20Object%20Reference%20%28by%20ref%29) (ForwardOffset :type Integer))
  (bind _returnvalue (Transformation|GetActorTransform User))
  (bind (_location _rotation _scale) (Math|Transform|BreakTransform _returnvalue))
  (return (Math|Transform|MakeTransform (+ (* (Transformation|GetActorForwardVector User) ForwardOffset) _location) _rotation _scale)))

(fn IsAbletoActivateforUserrrr?
  (params (User :type Skill%20Consumer%20Object%20Reference%20%28by%20ref%29))
  (Utilities|FlowControl|Sequence
    (:then_0
      (LocalVariables|SetRetval (Utilities|IsAbletoPayCost? User)))))

(fn SetupActivation
  (params (user :type Skill%20Consumer%20Object%20Reference%20%28by%20ref%29))
  (Utilities|IsAbletoActivateforUser? user
    (:True
      (LocalVariables|SetCurrent%20user user)
      (Utilities|FlowControl|Sequence
        (:then_0
          (bind _asplayer_character (Utilities|Casting|CastToPlayerCharacter (LocalVariables|GetCurrent%20user)))
          (Default|Root _asplayer_character (Variables|Default|GetRoot%20Time)))
        (:then_1
          (Utilities|SubtractSkillCost (LocalVariables|GetCurrent%20user)))
        (:then_2
          (return true))))
    (:False
      (return false))))