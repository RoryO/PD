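; Dummy cannon actor that repeatedly triggers a basic attack on a fixed timer, with no aiming or input.
; On BeginPlay it spawns a BasicAttack actor at its own transform as owner and instigator, stores it as AttackSkill, and starts a looping Fire timer.
; Fire sends the Activate message to that skill and resets the cannon's own life span, which outlasts the timer interval.
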(event EventBeginPlay
  (bind _self self)
  (bind _returnvalue (Game|SpawnActorfromClass "/Game/Blueprints/Projectile/Skills/BasicAttack.BasicAttack_C" (Transformation|GetActorTransform _self) "Undefined" _self 0.0 _self))
  (Variables|Default|SetAttackSkill _returnvalue)
  (Utilities|Time|SetTimerbyFunctionName 0 "Fire" 2.0 true))

(event Collision|EventActorBeginOverlap
  (params (OtherActor :type Actor%20Object%20Reference)))

(event EventTick
  (params (DeltaSeconds :type Float%20%28single-precision%29)))

(fn ConstructionScript)

(fn Fire
  (Class|ActivatedSkillInterface|Activate(Message) (Utilities|ToObject(Interface) (Variables|Default|GetAttackSkill)) self)
  (Actor|SetLifeSpan 5.0))