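; OtherCannon is a dummy actor that repeatedly fires the activated skill in its first slot.
; BeginPlay fills its skill points, resets the skill hand and starts a looping timer that calls Fire every two seconds.
; Fire casts the slot skill to ActivatedSkill and activates it on itself, while Tick keeps current skill points topped up so they never run out.
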(event EventBeginPlay
  (Variables|Default|SetCurrentSkillPoints 99)
  (Variables|Default|SetMaximumSkillPoints 99)
  (Default|ResetSkillHand self)
  (Utilities|Time|SetTimerbyFunctionName 0 "Fire" 2.0 true))

(event Collision|EventActorBeginOverlap
  (params (OtherActor :type Actor%20Object%20Reference)))

(event EventTick
  (params (DeltaSeconds :type Float%20%28single-precision%29))
  (Variables|Default|SetCurrentSkillPoints 99))

(fn ConstructionScript
  (|CallParentFunction))

(fn Fire
  (bind _asactivated_skill (Utilities|Casting|CastToActivatedSkill (CallFunction|GetSkillatSlot)))
  (Default|Activate _asactivated_skill self))