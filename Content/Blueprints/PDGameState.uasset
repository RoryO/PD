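; Game state Blueprint that picks the next target on the team opposing a given team.
; NextTargetForOppositeTeam selects TeamA or TeamB as the search set, then steps to the element after the current target.
; It returns the first element when the target is invalid or the set has one member.
; The wrap check compares the found index to array length, so the last element never wraps to the first.
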(event EventBeginPlay)

(event EventTick
  (params (DeltaSeconds :type Float%20%28single-precision%29)))

(fn ConstructionScript)

(fn NextTargetforOppositeTeam
  (params (Current%20Team :type Team%20Enum%20%28by%20ref%29) (Current%20Target :type Actor%20Object%20Reference))
  (Utilities|FlowControl|Sequence
    (:then_0
      (switch Utilities|FlowControl|Switch|SwitchonTeam Current%20Team
        (:NewEnumerator0
          (LocalVariables|SetSearch%20set (Variables|GameState|GetTeamB)))
        (:NewEnumerator1
          (LocalVariables|SetSearch%20set (Variables|GameState|GetTeamA)))))
    (:then_1
      (Utilities|IsValid Current%20Target ; If none, return first element
        (:Is%20Valid
          (if (== (Utilities|Array|Length (LocalVariables|GetSearch%20set)) 1)
            (Development|PrintString "2")
            (return (Utilities|Array|Get(acopy) (LocalVariables|GetSearch%20set)))
            (elif (== (Utilities|Array|Length (LocalVariables|GetSearch%20set)) (Utilities|Array|FindItem (LocalVariables|GetSearch%20set) Current%20Target))
              (Development|PrintString "3")
              (return (Utilities|Array|Get(acopy) (LocalVariables|GetSearch%20set)))
              (else
                (bind _output_get (LocalVariables|SetFoundIndex (Utilities|Array|FindItem (LocalVariables|GetSearch%20set) Current%20Target))) ; Goofy but using pure ++ does not work
                (bind _result (Math|Integer|IncrementInt _output_get)
                  (:%20%20
                    (return (Utilities|Array|Get(acopy) (LocalVariables|GetSearch%20set) _result))))))))
        (:Is%20Not%20Valid
          (Development|PrintString "1")
          (return (Utilities|Array|Get(acopy) (LocalVariables|GetSearch%20set))))))))