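; SkillConsumer manages a four-slot hand of skill actors and a discard pile.
; ResetSkillHand spawns a basic attack, a basic wall and two level-increase skills into the slots.
; DiscardSkill moves a skill to the discard pile and fills its slot with a lazily spawned, cached NullActivatedSkill.
; GetSkillAtSlot returns that same null-object placeholder for invalid slots, so lookups yield a skill actor.
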(event EventBeginPlay)

(event Collision|EventActorBeginOverlap
  (params (OtherActor :type Actor%20Object%20Reference)))

(event EventTick
  (params (DeltaSeconds :type Float%20%28single-precision%29)))

(fn ConstructionScript)

(fn ResetSkillHand
  (bind _self self)
  (bind _returnvalue (Transformation|GetActorTransform _self))
  (Utilities|Array|Resize (Variables|Default|GetSkillHand) 4)
  (Utilities|FlowControl|Sequence
    (:then_0
      (bind _returnvalue_2 (Game|SpawnActorfromClass "/Game/Blueprints/Projectile/Skills/BasicAttack.BasicAttack_C" _returnvalue "Undefined" 0 0.0 0))
      (Utilities|Array|SetArrayElem (Variables|Default|GetSkillHand) 0 _returnvalue_2))
    (:then_1
      (bind _returnvalue_3 (Game|SpawnActorfromClass "/Game/Blueprints/Wall/Skills/BasicWall.BasicWall_C" _returnvalue "Undefined" 0 0))
      (Utilities|Array|SetArrayElem (Variables|Default|GetSkillHand) 1 _returnvalue_3))
    (:then_2
      (bind _returnvalue_4 (Game|SpawnActorfromClass "/Game/Blueprints/Effect/Skills/SkillLevelIncrease.SkillLevelIncrease_C" _returnvalue "Undefined" 0 0))
      (Utilities|Array|SetArrayElem (Variables|Default|GetSkillHand) 2 _returnvalue_4))
    (:then_3
      (bind _returnvalue_5 (Game|SpawnActorfromClass "/Game/Blueprints/Effect/Skills/SkillLevelIncrease.SkillLevelIncrease_C" _returnvalue "Undefined" 0 0))
      (Utilities|Array|SetArrayElem (Variables|Default|GetSkillHand) 3 _returnvalue_5))))

(fn GetNullActivatedSkill
  (bind _self self)
  (Utilities|IsValid (Variables|Default|GetNullActivatedSkill)
    (:Is%20Valid
      (return (Variables|Default|GetNullActivatedSkill)))
    (:Is%20Not%20Valid
      (bind _returnvalue (Game|SpawnActorfromClass "/Game/Blueprints/NullActivatedSkill.NullActivatedSkill_C" (Transformation|GetActorTransform (Game|GetPlayerCharacter 0)) "Undefined" _self _self))
      (bind _output_get (Variables|Default|SetNullActivatedSkill _returnvalue))
      (return _output_get))))

(fn DiscardSkill
  (params (Skill :type Activated%20Skill%20Object%20Reference))
  (LocalVariables|SetActivated%20Skill Skill)
  (Utilities|FlowControl|Sequence
    (:then_0
      (LocalVariables|SetSkill%20Position%20Index (Utilities|Array|FindItem (Variables|Default|GetSkillHand) (LocalVariables|GetActivated%20Skill))))
    (:then_1
      (bind _nullactivatedskill (CallFunction|GetNullActivatedSkill))
      (Utilities|Array|SetArrayElem (Variables|Default|GetSkillHand) (LocalVariables|GetSkill%20Position%20Index) _nullactivatedskill))
    (:then_2
      (Utilities|Array|Add (Variables|Default|GetDiscardPile) (LocalVariables|GetActivated%20Skill)))))

(fn GetSkillatSlot
  (params (Slot :type Integer))
  (LocalVariables|SetFound%20Skill (Utilities|Array|Get(acopy) (Variables|Default|GetSkillHand) Slot))
  (if (Utilities|IsValid (LocalVariables|GetFound%20Skill))
    (return (LocalVariables|GetFound%20Skill))
    (else
      (bind _nullactivatedskill (CallFunction|GetNullActivatedSkill))
      (return _nullactivatedskill))))