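; Array utility functions for copying, distance sorting and nearest-actor lookup.
; Copy Array duplicates input element by element.
; Closest Actor from Actor compares location distances but keeps larger values, so it returns the farthest actor despite its name.
; The distance sort is unfinished: it returns arrays under two elements unchanged, leaves exactly two unhandled, and returns an unpopulated Sorted array for larger ones.
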(fn SortActorArraybyDistancefromActor
  (params (Current%20Array :type Array%20of%20Actor%20Object%20References) (Target%20Actor :type Actor%20Object%20Reference))
  (Math|Integer|CompareInt (Utilities|Array|Length Current%20Array) 2
    (:>
      (for _array_element Current%20Array
        (Utilities|IsValid (LocalVariables|GetHighest)
          (:Is%20Valid
            (if true
              _))
          (:Is%20Not%20Valid
            (LocalVariables|SetHighest (LocalVariables|GetHighest)))))
      (return (LocalVariables|GetSorted)))
    (:<
      (return Current%20Array))))

(fn CopyArray
  (params (In :type Array%20of%20Object%20Object%20References))
  (for _array_element In
    (Utilities|Array|Add (LocalVariables|GetCopy) _array_element))
  (return (LocalVariables|GetCopy)))

(fn ClosestActorfromActor
  (params (Actors :type Array%20of%20Actor%20Object%20References) (Source :type Actor%20Object%20Reference%20%28by%20ref%29))
  (for _array_element Actors
    (if (< (LocalVariables|GetShortest%20Distance) (Math|Vector|VectorLength (- (.Location (Math|Transform|BreakTransform (Transformation|GetActorTransform _array_element))) (.Location (Math|Transform|BreakTransform (Transformation|GetActorTransform Source))))))
      (LocalVariables|SetShortest%20Distance (Math|Vector|VectorLength (- (.Location (Math|Transform|BreakTransform (Transformation|GetActorTransform _array_element))) (.Location (Math|Transform|BreakTransform (Transformation|GetActorTransform Source))))))
      (LocalVariables|SetClosest%20Actor _array_element)))
  (return (LocalVariables|GetClosest%20Actor)))